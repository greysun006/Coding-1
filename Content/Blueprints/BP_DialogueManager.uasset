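; BP_DialogueManager shows timed lines of dialogue on screen, one per DisplayNextLine call.
; It creates a W_Dialogue widget at BeginPlay, then sets its text from the Dialogue array at the current Index.
; Each line stays in the viewport for five seconds, while Index advances without waiting for the delay.
; Past the last line, it restarts from the first if ShouldRepeatText is set, otherwise shows nothing.
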(event Custom|Display%20Next%20Line
  (bind _dialoguewidget (Variables|Default|GetDialogueWidget))
  (if (>= (Variables|Default|GetIndex) (Utilities|Array|Length (Variables|Default|GetDialogue))) ; IF the index is greater than\nor equal to the length of the\nDialogue Array, reset it
    (if (Variables|Default|GetShouldRepeatText)
      (Variables|Default|SetIndex 0)
      (Rendering|Components|TextRender|SetText (Variables|/Game/Widgets/W_Dialogue.W_Dialogue_C|GetTextBlock_0 (Variables|Default|GetDialogueWidget)) (Utilities|Array|Get(acopy) (Variables|Default|GetDialogue) (Variables|Default|GetIndex)) :!label _label)
      (Utilities|FlowControl|Sequence
        (:then_0
          (UserInterface|Viewport|AddtoViewport _dialoguewidget 0) ; Add the dialogue to the view
          (Utilities|FlowControl|Delay 5.0) ; Wait 5 seconds
          (Widget|RemovefromParent _dialoguewidget) ; Removes the dialogue from the viewport
        )
        (:then_1
          (Math|Integer|IncrementInt (Variables|Default|GetIndex)) ; Increment Int\nto add 1 to our index
        )))
    (else
      (goto _label))))

(event EventBeginPlay
  (bind _returnvalue (UserInterface|CreateWidget "/Game/Widgets/W_Dialogue.W_Dialogue_C")) ; Create widget
  (Variables|Default|SetDialogueWidget _returnvalue))

(fn ConstructionScript)