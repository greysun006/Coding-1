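; BP_Cannon is a cannon actor that automatically fires a cannonball once per second from BeginPlay onward.
; A Delay wired back into itself calls FireCannon, which spawns a BP_CannonBall at the SpawnPoint component's world transform.
; Each new ball's Sphere gets a single large AddForce along SpawnPoint's forward vector, applied as an acceleration change so the launch ignores mass.
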(event Custom|Fire%20Cannon
  (bind _returnvalue (Game|SpawnActorfromClass "/Game/Blueprints/BP_CannonBall.BP_CannonBall_C" (Transformation|GetWorldTransform (Variables|Default|GetSpawnPoint)) "Undefined" "MultiplyWithRoot" 0 0)) ; Spawn Actor from Class
  (Physics|AddForce (Variables|/Game/Blueprints/BP_CannonBall.BP_CannonBall_C|GetSphere _returnvalue) (* (Math|Vector|GetForwardVector (Variables|Default|GetSpawnPoint)) 1e+05) "None" true))

(event EventBeginPlay
  (Utilities|FlowControl|Delay 1.0 :!label _label)
  (CallFunction|FireCannon)
  (goto _label))

(fn ConstructionScript)