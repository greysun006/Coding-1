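; BP_Tree is a tree actor that picks a random static mesh at BeginPlay and grows in timed steps.
; A delayed DoN loop runs a random number of times, each pass adding a random amount to the mesh's relative scale.
; After the last growth step, it enables query and physics collision on the mesh.
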(event Custom|Grow
  (bind _sm_tree (Variables|Default|GetSM_Tree))
  (Transformation|SetRelativeScale3D _sm_tree (+ (Variables|/Script/Engine.SceneComponent|GetRelativeScale3D _sm_tree) (Math|Random|RandomFloatinRange 0.2 0.4))))

(event Custom|The%20Grow%20Loop
  (bind _output_get (Variables|Default|SetLoopCount (Math|Random|RandomIntegerinRange 1 5)))
  (bind _counter (Utilities|FlowControl|DoN _output_get :!label _label)
    (:Exit
      (Utilities|FlowControl|Delay (Math|Random|RandomFloatinRange 3.0 5.0))
      (CallFunction|Grow)
      (if (== _counter _output_get)
        (Collision|SetCollisionEnabled (Variables|Default|GetSM_Tree) "QueryAndPhysics")
        (else
          (goto _label))))))

(event EventBeginPlay
  (Components|StaticMesh|SetStaticMesh (Variables|Default|GetSM_Tree) (.OutItem (Utilities|Array|Random (Variables|Default|GetNew%20Mesh))))
  (CallFunction|TheGrowLoop))

(fn ConstructionScript)