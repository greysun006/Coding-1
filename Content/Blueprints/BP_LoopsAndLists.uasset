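; Loop demonstration Blueprint that randomly rotates every BP_Rat on all axes every 0.7 seconds from BeginPlay via a self-repeating Delay.
; LoopArrayOverTime spreads an array loop over time with an index and Delay, randomly yawing shuffled BP_Tree actors one by one.
; Its only caller is a disconnected repeating timer chain, and a colored countdown while loop is also unwired.
; SimpleLoop and WhileLoopFunction are called at BeginPlay but are empty.
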(event Custom|Rat%20Loop
  (Utilities|FlowControl|Delay 0.7 :!label _label)
  (CallFunction|SpintheRat)
  (goto _label))

(event Custom|WhileLoop%20Function)

(event Custom|Spin%20The%20Rat
  (bind _returnvalue (Math|Random|RandomFloatinRange 0.0 3.6e+02))
  (bind _outactors (Actor|GetAllActorsOfClass "/Game/Blueprints/BP_Rat.BP_Rat_C"))
  (for _array_element _outactors
    (Transformation|SetActorRelativeRotation _array_element (Math|Rotator|MakeRotator _returnvalue _returnvalue _returnvalue))))

(event Custom|Simple%20Loop)

(event Custom|Loop%20Array%20Over%20Time
  (bind _outactors (Actor|GetAllActorsOfClass "/Game/Blueprints/BP_Tree.BP_Tree_C"))
  (Utilities|Array|Shuffle _outactors)
  (if (< (Variables|Default|GetOvertimeIndex) (Utilities|Array|Length _outactors)) :!label _label ; Test for our loop.
    (Transformation|SetActorRelativeRotation (Utilities|Array|Get(acopy) _outactors (Variables|Default|GetOvertimeIndex)) (Math|Rotator|MakeRotator 0.0 0.0 (Math|Random|RandomFloatinRange 0.0 3.6e+02)))
    (Math|Integer|IncrementInt (Variables|Default|GetOvertimeIndex)
      (:%20%20
        (Utilities|FlowControl|Delay 0.2)
        (goto _label)))
    (else
      (Variables|Default|SetOvertimeIndex 0))))

(event EventBeginPlay
  (CallFunction|SimpleLoop)
  (CallFunction|WhileLoopFunction)
  (CallFunction|RatLoop))

(fn ConstructionScript)